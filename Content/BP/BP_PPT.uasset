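; BP_PPT is a presentation actor that shows slides and a progress bar timing the leader's turns between facing the PPT and facing the player.
; Tick advances a timer, feeds it to the WBP_Counter widget and flips the Face state when each phase's duration ends.
; Durations come from the first BP_Leader_L2, with a fixed offset on slide time for delay and rotation.
; A RepNotify on CurrentSlideIndex updates the WBP_PPT slide widget.
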(event `self.ReceiveBeginPlay`
  (set `self.Current Time` 0.0)
  (`self.UpdateTime`))

(event `self.ReceiveTick`
  (params (DeltaSeconds :type "Float (single-precision)"))
  ; 转头正计时，currentTime是当前处于这个状态多少秒，backTime是
  (if (< (`self.Current Time`) (`self.Back Time`))
    (set `self.Current Time` (+ (`self.Current Time`) DeltaSeconds))
    (if (`self.Face?`)
      (`self.UpdateTime`)
      (else
        (`self.UpdateFacetime`)))
    (else
      (set `self.Current Time` 0.0))))

(event `UpdateTime`
  ; 面向PPT的时间进度条显示
  (bind _aswbp_counter (cast `/Game/BP/WBP/WBP_Counter` (`WidgetComponent.GetUserWidgetObject` (`self.Widget`))))
  (set `/Game/BP/WBP/WBP_Counter.currentTime` (`self.Current Time`) _aswbp_counter)
  (bind _outactors (`GameplayStatics.GetAllActorsOfClass` "/Game/Characters/BP_Leader_L2.BP_Leader_L2_C"))
  (bind _returnvalue (+ (`/Game/Characters/BP_Leader_L2.TimePerSlide` (`|GetArrayItem` _outactors)) 4.4))
  (set `/Game/BP/WBP/WBP_Counter.totalTime` _returnvalue _aswbp_counter)
  (set `self.Back Time` _returnvalue)
  (if (not (< (`self.Current Time`) (`self.Back Time`)))
    (set `self.Face?` false)))

(event `UpdateFacetime`
  ; 面向玩家的时间进度条显示
  (bind _aswbp_counter (cast `/Game/BP/WBP/WBP_Counter` (`WidgetComponent.GetUserWidgetObject` (`self.Widget`))))
  (set `/Game/BP/WBP/WBP_Counter.currentTime` (`self.Current Time`) _aswbp_counter)
  (bind _outactors (`GameplayStatics.GetAllActorsOfClass` "/Game/Characters/BP_Leader_L2.BP_Leader_L2_C"))
  (bind _checkplayertime (`/Game/Characters/BP_Leader_L2.CheckPlayerTime` (`|GetArrayItem` _outactors)))
  (set `/Game/BP/WBP/WBP_Counter.totalTime` _checkplayertime _aswbp_counter)
  (set `self.Back Time` _checkplayertime)
  (if (not (< (`self.Current Time`) (`self.Back Time`)))
    (set `self.Face?` true)))

(fn `OnRep_CurrentSlideIndex`
  (bind _aswbp_ppt (cast `/Game/BP/WBP/WBP_PPT` (`WidgetComponent.GetUserWidgetObject` (`self.PPT`))))
  (`/Game/BP/WBP/WBP_PPT.UPdate` _aswbp_ppt (`self.CurrentSlideIndex`)))

(fn `UserConstructionScript`)