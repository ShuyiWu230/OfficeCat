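; BP_HideZone is a trigger volume that hides the player from the BP_Leader_L2 actor while they stand inside it.
; On BeginPlay it caches the first BP_Leader_L2 found in the level via GetAllActorsOfClass.
; Box overlap events from BP_ThirdPersonCharacter set the leader's CanSeePlayerOverride to false on entry and back to true on exit.
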(event `self.ReceiveBeginPlay`
  (bind _outactors (`GameplayStatics.GetAllActorsOfClass` "/Game/Characters/BP_Leader_L2.BP_Leader_L2_C"))
  (bind _asbp_leader_l2 (cast `/Game/Characters/BP_Leader_L2` (`|GetArrayItem` _outactors)))
  (set `self.LeaderRef` _asbp_leader_l2))

(event `self.Box.OnComponentBeginOverlap`
  (params (OverlappedComponent :type "PrimitiveComponent Object Reference") (OtherActor :type "Actor Object Reference") (OtherComp :type "PrimitiveComponent Object Reference") (OtherBodyIndex :type Integer) (bFromSweep :type Boolean) (SweepResult :type "HitResult Structure (by ref)"))
  (cast `/Game/ThirdPerson/Blueprints/BP_ThirdPersonCharacter` OtherActor)
  (set `/Game/Characters/BP_Leader_L2.CanSeePlayerOverride` false (`self.LeaderRef`)))

(event `self.Box.OnComponentEndOverlap`
  (params (OverlappedComponent :type "PrimitiveComponent Object Reference") (OtherActor :type "Actor Object Reference") (OtherComp :type "PrimitiveComponent Object Reference") (OtherBodyIndex :type Integer))
  (cast `/Game/ThirdPerson/Blueprints/BP_ThirdPersonCharacter` OtherActor)
  (set `/Game/Characters/BP_Leader_L2.CanSeePlayerOverride` true (`self.LeaderRef`)))

(fn `UserConstructionScript`)