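; Cat NPC that patrols, follows a player holding a cat toy, and can be caught.
; A looping timer checks toy and distance, switching AIMoveTo between the nearby player and looping patrol points with per-point waits, gated by IsBusy.
; Player overlap with the sphere shows a progress widget that Tick fills; leaving resets the timer.
; A full bar destroys the cat and sets HaveCat on the player.
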(event `self.ReceiveBeginPlay`
  (`KismetSystemLibrary.K2_SetTimerDelegate` (delegate `CheckCatToy`) 0.25 true)
  (`self.Move`)
  (bind _aswbp_cat (cast `/Game/BP/WBP/WBP_Cat` (`WidgetComponent.GetUserWidgetObject` (`self.Widget`))))
  (set `self.CatWidgetRef` _aswbp_cat))

(event `CheckCatToy`
  ; 逗猫棒
  (bind _asbp_third_person_character (cast `/Game/ThirdPerson/Blueprints/BP_ThirdPersonCharacter` (`GameplayStatics.GetPlayerCharacter` 0)))
  (if (and (< (`KismetMathLibrary.Vector_Distance` (`self.K2_GetActorLocation` _asbp_third_person_character) (`self.K2_GetActorLocation`)) 350.0) (`/Game/ThirdPerson/Blueprints/BP_ThirdPersonCharacter.HoldCatToy` _asbp_third_person_character))
    (`|ExecutionSequence`
      (:`then_0`
        (`/Engine/EditorBlueprintResources/StandardMacros.DoOnce` false :!label _label
          (:`Completed`
            (`MovementComponent.StopMovementImmediately` (`self.CharacterMovement`)))))
      (:`then_1`
        (set `self.isBusy?` true)
        (`|AIMoveTo` self (0.0 0.0 0.0) (`GameplayStatics.GetPlayerCharacter` 0) 100.0
          (:`OnSuccess`
            _)
          (:`OnFail`
            _))
        (set `self.isBusy?` false)))
    (else
      (`|ExecutionSequence`
        (:`then_0`
          (goto _label :!via `Reset`))
        (:`then_1`
          (if (not (`self.isBusy?`))
            (`self.Move`)))))))

(event `Move`
  ; 小猫巡逻
  (set `self.isBusy?` true)
  (`|AIMoveTo` self (0.0 0.0 0.0) (`|GetArrayItem` (`self.PatrolPoint`) (`self.CurrentPatrolIndex`))
    (:`OnSuccess`
      (`KismetSystemLibrary.Delay` (`|GetArrayItem` (`self.WaitTime`) (`self.CurrentPatrolIndex`)))
      (`/Engine/EditorBlueprintResources/StandardMacros.IncrementInt` (`self.CurrentPatrolIndex`)
        (:`  `
          (if (<= (`self.CurrentPatrolIndex`) (`KismetArrayLibrary.Array_LastIndex` (`self.PatrolPoint`)))
            (set `self.isBusy?` false)
            (else
              (set `self.CurrentPatrolIndex` 0)
              (set `self.isBusy?` false))))))
    (:`OnFail`
      (set `self.isBusy?` false))))

(event `self.Sphere.OnComponentBeginOverlap`
  (params (OverlappedComponent :type "PrimitiveComponent Object Reference") (OtherActor :type "Actor Object Reference") (OtherComp :type "PrimitiveComponent Object Reference") (OtherBodyIndex :type Integer) (bFromSweep :type Boolean) (SweepResult :type "HitResult Structure (by ref)"))
  ; 抓猫
  (bind _asbp_third_person_character (cast `/Game/ThirdPerson/Blueprints/BP_ThirdPersonCharacter` OtherActor))
  (set `self.bIsCatching` true)
  ;; 进度条出现
  (`Widget.SetVisibility` (`self.CatWidgetRef`) "Visible"))

(event `self.Sphere.OnComponentEndOverlap`
  (params (OverlappedComponent :type "PrimitiveComponent Object Reference") (OtherActor :type "Actor Object Reference") (OtherComp :type "PrimitiveComponent Object Reference") (OtherBodyIndex :type Integer))
  ; 抓猫
  (cast `/Game/ThirdPerson/Blueprints/BP_ThirdPersonCharacter` OtherActor)
  (set `self.bIsCatching` false)
  (set `self.CatchingCurrentTime` 0.0)
  ;; 进度条消失
  (`Widget.SetVisibility` (`self.CatWidgetRef`) "Hidden"))

(event `self.ReceiveTick`
  (params (DeltaSeconds :type "Float (single-precision)"))
  ; 抓猫
  (if (`self.bIsCatching`)
    ;; 把抓猫进度推送给UI进度条
    (set `self.CatchingCurrentTime` (+ (`self.CatchingCurrentTime`) (`GameplayStatics.GetWorldDeltaSeconds`)))
    (bind _output_get (set `self.Progress` (/ (`self.CatchingCurrentTime`) (`self.CatchingTotalTime`))))
    (`/Game/BP/WBP/WBP_Cat.SetCatchProgress` (`self.CatWidgetRef`) _output_get)
    (if (>= (`self.CatchingCurrentTime`) (`self.CatchingTotalTime`))
      (`self.K2_DestroyActor`)
      (set `/Game/ThirdPerson/Blueprints/BP_ThirdPersonCharacter.haveCat?` true (stale `self.Sphere.OnComponentBeginOverlap` _asbp_third_person_character))
      (`KismetSystemLibrary.PrintString` "抓到猫了"))))

(fn `UserConstructionScript`)