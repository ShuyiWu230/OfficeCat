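; BP_Leader is a watcher character that periodically turns around and checks whether a player character it sees is sitting down.
; A self-rescheduling Rotate timer flips it 180 degrees and toggles BisfacingPpl, alternating between the Time and BackTime delays.
; PawnSensing's see event reads SitDown on BP_ThirdPersonCharacter and only prints "无事发生" (nothing happens) if seated, otherwise "死" (die).
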(event `self.ReceiveBeginPlay`
  (`KismetSystemLibrary.K2_SetTimer` null "Rotate" (`self.Time`)))

(event `self.PawnSensing.OnSeePawn`
  (params (Pawn :type "Pawn Object Reference"))
  (bind _asbp_third_person_character (cast `/Game/ThirdPerson/Blueprints/BP_ThirdPersonCharacter` Pawn))
  (if (`/Game/ThirdPerson/Blueprints/BP_ThirdPersonCharacter.SitDown` _asbp_third_person_character)
    (`KismetSystemLibrary.PrintString` "无事发生")
    (else
      (`KismetSystemLibrary.PrintString` "死"))))

(fn `Rotate`
  (`self.K2_AddActorLocalRotation` (struct :`Yaw` 180.0))
  (set `self.bisfacingPpl` (not (`self.bisfacingPpl`)))
  (if (`self.bisfacingPpl`)
    (`KismetSystemLibrary.K2_SetTimer` null "Rotate" (`self.BackTime`))
    (else
      (`KismetSystemLibrary.K2_SetTimer` null "Rotate" (`self.Time`)))))

(fn `UserConstructionScript`)